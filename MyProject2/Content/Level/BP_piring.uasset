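; BP_piring is a plate actor that receives a fried egg from a BP_pan in a cooking level.
; While something overlaps its Box, component activation drives a short delay loop that runs activate, sphere-tracing at the plate until it holds an egg.
; A filled pan's egg is hidden and the plate's shown, printing a win message if doneness is near full.
; Hit actors that are not pans get added to the trace's ignore list.
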(event OnComponentEndOverlap(Box)
  (params (OverlappedComponent :type Primitive%20Component%20Object%20Reference) (OtherActor :type Actor%20Object%20Reference) (OtherComp :type Primitive%20Component%20Object%20Reference) (OtherBodyIndex :type Integer))
  (Variables|Default|SetinRadius false)
  (Components|Activation|Deactivate (Variables|Default|GetBox)))

(event OnComponentActivated(Box)
  (params (Component :type Actor%20Component%20Object%20Reference) (bReset :type Boolean))
  (if (Variables|Default|GetinRadius) :!label _label
    (CallFunction|Activate)
    (Utilities|FlowControl|Delay 0.1)
    (goto _label)))

(event OnComponentBeginOverlap(Box)
  (params (OverlappedComponent :type Primitive%20Component%20Object%20Reference) (OtherActor :type Actor%20Object%20Reference) (OtherComp :type Primitive%20Component%20Object%20Reference) (OtherBodyIndex :type Integer) (bFromSweep :type Boolean) (SweepResult :type Hit%20Result%20Structure%20%28by%20ref%29))
  (Variables|Default|SetinRadius true)
  (Components|Activation|Activate (Variables|Default|GetBox) false))

(event Custom|activate
  (bind _plate (Variables|Default|GetPlate))
  (bind _returnvalue (Transformation|GetWorldLocation _plate))
  (if (not (Variables|Default|Getadatelur))
    (bind _outhit (Collision|SphereTraceForObjects _returnvalue _returnvalue 1e+02 (Variables|Default|GetObject%20Types) false (Variables|Default|GetActors%20to%20Ignore) "ForDuration"))
    (Utilities|IsValid (.HitActor (Collision|BreakHitResult _outhit))
      (:Is%20Valid
        (bind _asbp_pan (Utilities|Casting|CastToBP_pan (.HitActor (Collision|BreakHitResult _outhit)))
          (:then
            (if (Variables|/Game/Level/BP_pan.BP_pan_C|Getadakonten _asbp_pan)
              (Development|PrintString "isi")
              (Rendering|SetVisibility (Variables|/Game/Level/BP_pan.BP_pan_C|Getsunny%20side%20up%20egg _asbp_pan) false true)
              (Rendering|SetVisibility (Variables|Default|GetSunny%20Side%20Up%20Egg) true true)
              (Variables|/Game/Level/BP_pan.BP_pan_C|Setadakonten _asbp_pan false)
              (Variables|Default|Setadatelur true)
              (if (> (Variables|/Game/Level/BP_pan.BP_pan_C|Getdoneness _asbp_pan) 99.0)
                (Development|PrintString "you win"))))
          (:CastFailed
            (Utilities|Array|Add (Variables|Default|GetActors%20to%20Ignore) (.HitActor (Collision|BreakHitResult _outhit)))))))))

(event EventBeginPlay)

(event Collision|EventActorBeginOverlap
  (params (OtherActor :type Actor%20Object%20Reference)))

(event EventTick
  (params (DeltaSeconds :type Float%20%28single-precision%29)))

(fn ConstructionScript)