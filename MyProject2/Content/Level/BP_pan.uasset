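; BP_pan is a cooking pan that accepts an egg and cooks it on the stove.
; An InputBox overlap sphere-traces around the pan, adding non-egg hits to an ignore list and retrying after a delay.
; If empty, it destroys an ungrabbed egg and reveals the SunnySideUpEgg component.
; While DiatasKompor (on stove) is true, Tick switches collision type and adds Heat to Doneness, regardless of contents.
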(event OnComponentBeginOverlap(inputbox)
  (params (OverlappedComponent :type Primitive%20Component%20Object%20Reference) (OtherActor :type Actor%20Object%20Reference) (OtherComp :type Primitive%20Component%20Object%20Reference) (OtherBodyIndex :type Integer) (bFromSweep :type Boolean) (SweepResult :type Hit%20Result%20Structure%20%28by%20ref%29))
  (bind _actors_to_ignore_0 (Variables|Default|GetActors%20to%20Ignore_0))
  (bind _pan (Variables|Default|Getpan))
  (bind _returnvalue (Transformation|GetWorldLocation _pan))
  (Variables|Default|SetinRadius true)
  (bind _outhit (Collision|SphereTraceForObjects _returnvalue _returnvalue 2e+02 (Variables|Default|GetObject%20Types) false _actors_to_ignore_0 "ForDuration" :!label _label))
  (Utilities|IsValid (.HitActor (Collision|BreakHitResult _outhit))
    (:Is%20Valid
      (bind _asbp_egg (Utilities|Casting|CastToBP_egg (.HitActor (Collision|BreakHitResult _outhit)))
        (:then
          (if (Variables|/Game/Level/BP_egg.BP_egg_C|Getgrabbed _asbp_egg)
            (Development|PrintString "grabbed")
            (elif (Variables|Default|Getadakonten)
              (Development|PrintString "Hello")
              (else
                (Actor|DestroyActor _asbp_egg)
                (Rendering|SetVisibility (Variables|Default|Getsunny%20side%20up%20egg) true true)
                (Development|PrintString "telur masuk")
                (Variables|Default|Setadakonten true)))))
        (:CastFailed
          (Utilities|Array|Add _actors_to_ignore_0 (.HitActor (Collision|BreakHitResult _outhit)))
          (Utilities|FlowControl|Delay 0.2)
          (goto _label))))))

(event OnComponentEndOverlap(inputbox)
  (params (OverlappedComponent :type Primitive%20Component%20Object%20Reference) (OtherActor :type Actor%20Object%20Reference) (OtherComp :type Primitive%20Component%20Object%20Reference) (OtherBodyIndex :type Integer))
  (Variables|Default|SetinRadius false))

(event EventBeginPlay)

(event Collision|EventActorBeginOverlap
  (params (OtherActor :type Actor%20Object%20Reference)))

(event EventTick
  (params (DeltaSeconds :type Float%20%28single-precision%29))
  (bind _pan (Variables|Default|Getpan))
  (if (Variables|Default|GetdiatasKompor)
    (Collision|SetCollisionObjectType _pan "ECC_PhysicsBody")
    (bind _output_get (Variables|Default|Setdoneness (+ (Variables|Default|Getdoneness) (Variables|Default|Getheat))))
    (Development|PrintString (Utilities|String|ToString(Float) _output_get))
    (else
      (Collision|SetCollisionObjectType _pan "ECC_Pawn"))))

(fn ConstructionScript)