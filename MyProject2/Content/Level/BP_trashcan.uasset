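; BP_trashcan is a trashcan actor that disposes of eggs dropped into its Box collider.
; On Box overlap, a cast chain ignores both Leap hands (BP_leapKiri, BP_leapkanan) and destroys any BP_egg that is not grabbed; the BP_pan branch is empty.
; Tick looks up and stores both hand actors every frame, though nothing here reads them, and Box hits only print a debug string.
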(event OnComponentBeginOverlap(Box)
  (params (OverlappedComponent :type Primitive%20Component%20Object%20Reference) (OtherActor :type Actor%20Object%20Reference) (OtherComp :type Primitive%20Component%20Object%20Reference) (OtherBodyIndex :type Integer) (bFromSweep :type Boolean) (SweepResult :type Hit%20Result%20Structure%20%28by%20ref%29))
  (Utilities|Casting|CastToBP_leapKiri OtherActor
    (:CastFailed
      (Utilities|Casting|CastToBP_leapkanan OtherActor
        (:CastFailed
          (bind _asbp_egg (Utilities|Casting|CastToBP_egg OtherActor)
            (:then
              (if (not (Variables|/Game/Level/BP_egg.BP_egg_C|Getgrabbed _asbp_egg))
                (Actor|DestroyActor OtherActor)))
            (:CastFailed
              (Utilities|Casting|CastToBP_pan OtherActor))))))))

(event OnComponentHit(Box)
  (params (HitComponent :type Primitive%20Component%20Object%20Reference) (OtherActor :type Actor%20Object%20Reference) (OtherComp :type Primitive%20Component%20Object%20Reference) (NormalImpulse :type Vector :default "0, 0, 0") (Hit :type Hit%20Result%20Structure%20%28by%20ref%29))
  (Development|PrintString "Hello"))

(event EventBeginPlay)

(event Collision|EventActorBeginOverlap
  (params (OtherActor :type Actor%20Object%20Reference)))

(event EventTick
  (params (DeltaSeconds :type Float%20%28single-precision%29))
  (bind _returnvalue (Actor|GetActorOfClass "/Game/Level/BP_leapkanan.BP_leapkanan_C"))
  (Variables|Default|Setkanan _returnvalue)
  (bind _returnvalue_2 (Actor|GetActorOfClass "/Game/Level/BP_leapKiri.BP_leapKiri_C"))
  (Variables|Default|Setkiri _returnvalue_2))

(fn ConstructionScript)