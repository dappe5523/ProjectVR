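; Left-hand Leap Motion actor that lets the player grab and carry cube, pan and egg objects.
; Tracking data moves its skeletal mesh to the axis-remapped, scaled palm position.
; A left-hand grab sphere-traces at the mesh, and a short Delay loop pins the hit component to the hand with gravity off.
; Any hand release ends the loop, restoring gravity and clearing the egg's grabbed flag.
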(event OnLeapTrackingData(Leap)
  (params (Frame :type Leap%20Frame%20Data%20Structure%20%28by%20ref%29))
  (for _array_element (.Hands (Utilities|Struct|BreakLeapFrameData Frame))
    (switch Utilities|FlowControl|Switch|SwitchonEHandType (.HandType (Utilities|Struct|BreakLeapHandData _array_element))
      (:LEAP_HAND_LEFT
        (Variables|Default|Sethand _array_element))))
  (Transformation|SetWorldLocation (Variables|Default|GetSkeletalMesh) (* (Math|Vector|MakeVector (.z (.Position (Utilities|Struct|BreakLeapPalmData (.Palm (Utilities|Struct|BreakLeapHandData (Variables|Default|Gethand)))))) (* (.y (.Position (Utilities|Struct|BreakLeapPalmData (.Palm (Utilities|Struct|BreakLeapHandData (Variables|Default|Gethand)))))) -1.0) (.x (.Position (Utilities|Struct|BreakLeapPalmData (.Palm (Utilities|Struct|BreakLeapHandData (Variables|Default|Gethand))))))) (Variables|Default|GetMulttangan)) false false)
  (Variables|Default|SetHand%20Pos (* (Math|Vector|MakeVector (.z (.Position (Utilities|Struct|BreakLeapPalmData (.Palm (Utilities|Struct|BreakLeapHandData (Variables|Default|Gethand)))))) (* (.y (.Position (Utilities|Struct|BreakLeapPalmData (.Palm (Utilities|Struct|BreakLeapHandData (Variables|Default|Gethand)))))) -1.0) (.x (.Position (Utilities|Struct|BreakLeapPalmData (.Palm (Utilities|Struct|BreakLeapHandData (Variables|Default|Gethand))))))) (Variables|Default|GetMulttangan))))

(event OnHandGrabbed(Leap)
  (params (Hand :type Leap%20Hand%20Data%20Structure%20%28by%20ref%29))
  (bind _skeletalmesh (Variables|Default|GetSkeletalMesh))
  (bind _returnvalue (Transformation|GetWorldLocation _skeletalmesh))
  (switch Utilities|FlowControl|Switch|SwitchonEHandType (.HandType (Utilities|Struct|BreakLeapHandData Hand))
    (:LEAP_HAND_LEFT
      (Variables|Default|Setgrabbed true)
      (bind (_outhit _returnvalue_2) (Collision|SphereTraceForObjects _returnvalue _returnvalue 1e+02 (Variables|Default|GetObject%20Types) false 0 "ForDuration"))
      (if _returnvalue_2
        (bind _asbp_cube (Utilities|Casting|CastToBP_cube (.HitActor (Collision|BreakHitResult _outhit)))
          (:then
            (CallFunction|MoveObject (Variables|/Game/Level/BP_cube.BP_cube_C|GetCube1 _asbp_cube)))
          (:CastFailed
            (bind _asbp_pan (Utilities|Casting|CastToBP_pan (.HitActor (Collision|BreakHitResult _outhit)))
              (:then
                (CallFunction|MoveObject (Variables|/Game/Level/BP_pan.BP_pan_C|Gethead _asbp_pan)))
              (:CastFailed
                (bind _asbp_egg (Utilities|Casting|CastToBP_egg (.HitActor (Collision|BreakHitResult _outhit))))
                (Variables|/Game/Level/BP_egg.BP_egg_C|Setgrabbed _asbp_egg true)
                (CallFunction|MoveObject (Variables|/Game/Level/BP_egg.BP_egg_C|Getegg _asbp_egg) _asbp_egg)))))))))

(event OnHandReleased(Leap)
  (params (Hand :type Leap%20Hand%20Data%20Structure%20%28by%20ref%29))
  (Variables|Default|Setgrabbed false))

(event Custom|moveObject
  (params (targetObject :type Static%20Mesh%20Component%20Object%20Reference) (targetActor :type Actor%20Object%20Reference))
  (Utilities|IsValid targetObject :!label _label
    (:Is%20Valid
      (if (Variables|Default|Getgrabbed)
        (Transformation|SetWorldLocation targetObject (Variables|Default|GetHand%20Pos) false false)
        (Physics|SetEnableGravity targetObject false)
        (Utilities|FlowControl|Delay 0.001)
        (goto _label)
        (else
          (Physics|SetEnableGravity targetObject true)
          (Utilities|IsValid targetActor
            (:Is%20Valid
              (bind _asbp_egg (Utilities|Casting|CastToBP_egg targetActor))
              (Variables|/Game/Level/BP_egg.BP_egg_C|Setgrabbed _asbp_egg false))))))))

(event EventBeginPlay)

(event Collision|EventActorBeginOverlap
  (params (OtherActor :type Actor%20Object%20Reference)))

(event EventTick
  (params (DeltaSeconds :type Float%20%28single-precision%29)))

(fn ConstructionScript)