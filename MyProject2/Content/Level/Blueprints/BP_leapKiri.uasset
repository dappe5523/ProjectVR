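; Leap Motion left-hand actor that lets the player grab and operate kitchen objects.
; Tracking frames animate the hand mesh and place it relative to the player camera.
; On grab, a sphere trace picks up cubes, eggs, pans or plates, spawns new ones from racks, or toggles stove knobs.
; Delay loops pin held objects to the hand, tilting pans with it, and restore physics on release.
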(event OnLeapTrackingData(Leap)
  (params (Frame :type Leap%20Frame%20Data%20Structure%20%28by%20ref%29))
  (bind _multtangan (Variables|Default|GetMulttangan))
  (bind _as_bp_player (Variables|Default|GetAs%20BP%20Player))
  (bind _distance_to_player (Variables|Default|Getdistance%20to%20player))
  (bind _camera (Variables|/Game/Level/Blueprints/BP_player.BP_player_C|GetCamera _as_bp_player))
  (bind _returnvalue (Math|Vector|GetForwardVector _camera))
  (bind _returnvalue_2 (Transformation|GetWorldLocation _camera))
  (bind _returnvalue_3 (Transformation|GetWorldRotation _camera))
  (bind _returnvalue_4 (* _returnvalue _distance_to_player))
  (bind _returnvalue_5 (+ _returnvalue_4 _returnvalue_2))
  (for _array_element (.Hands (Utilities|Struct|BreakLeapFrameData Frame))
    (switch Utilities|FlowControl|Switch|SwitchonEHandType (.HandType (Utilities|Struct|BreakLeapHandData _array_element))
      (:LEAP_HAND_LEFT
        (CallFunction|SetLeftanim _array_element)
        (bind _output_get (Variables|Default|Sethand _array_element))
        (if (.IsExtended (Utilities|Struct|BreakLeapDigitData (.Index (Utilities|Struct|BreakLeapHandData _output_get))))
          _))))
  (Transformation|SetWorldLocation (Variables|Default|GetSkeletalMesh) (+ (Math|Vector|MakeVector (.x _returnvalue_5) (.y _returnvalue_5) (- (.z _returnvalue_5) 5e+02)) (* (Math|Vector|RotateVector (Math|Vector|MakeVector (.z (.Position (Utilities|Struct|BreakLeapPalmData (.Palm (Utilities|Struct|BreakLeapHandData (Variables|Default|Gethand)))))) (* (.y (.Position (Utilities|Struct|BreakLeapPalmData (.Palm (Utilities|Struct|BreakLeapHandData (Variables|Default|Gethand)))))) -1.0) (.x (.Position (Utilities|Struct|BreakLeapPalmData (.Palm (Utilities|Struct|BreakLeapHandData (Variables|Default|Gethand))))))) (Transformation|GetWorldRotation _camera)) (Math|Vector|MakeVector _multtangan _multtangan 2e+01))) false false)
  (Variables|Default|SetHand%20Pos (+ (Math|Vector|MakeVector (.x _returnvalue_5) (.y _returnvalue_5) (- (.z _returnvalue_5) 5e+02)) (* (Math|Vector|RotateVector (Math|Vector|MakeVector (.z (.Position (Utilities|Struct|BreakLeapPalmData (.Palm (Utilities|Struct|BreakLeapHandData (Variables|Default|Gethand)))))) (* (.y (.Position (Utilities|Struct|BreakLeapPalmData (.Palm (Utilities|Struct|BreakLeapHandData (Variables|Default|Gethand)))))) -1.0) (.x (.Position (Utilities|Struct|BreakLeapPalmData (.Palm (Utilities|Struct|BreakLeapHandData (Variables|Default|Gethand))))))) (Transformation|GetWorldRotation _camera)) (Math|Vector|MakeVector _multtangan _multtangan 2e+01))))
  (Transformation|SetWorldRotation (Variables|Default|GetSkeletalMesh) (Math|Rotator|MakeRotator (+ (.roll _returnvalue_3) 3e+01) (+ (.pitch _returnvalue_3) 9e+01) (+ (.yaw _returnvalue_3) 1.8e+02)) false false))

(event OnHandGrabbed(Leap)
  (params (Hand :type Leap%20Hand%20Data%20Structure%20%28by%20ref%29))
  (bind _returnvalue (Transformation|GetActorTransform))
  (bind _skeletalmesh (Variables|Default|GetSkeletalMesh))
  (bind _returnvalue_2 (Transformation|GetWorldLocation _skeletalmesh))
  (switch Utilities|FlowControl|Switch|SwitchonEHandType (.HandType (Utilities|Struct|BreakLeapHandData Hand))
    (:LEAP_HAND_LEFT
      (Variables|Default|Setgrabbed true)
      (bind (_outhit _returnvalue_3) (Collision|SphereTraceForObjects _returnvalue_2 _returnvalue_2 1e+02 (Variables|Default|GetObject%20Types) false 0 "ForDuration"))
      (if _returnvalue_3
        (bind _asbp_cube (Utilities|Casting|CastToBP_cube (.HitActor (Collision|BreakHitResult _outhit)))
          (:then
            (CallFunction|MoveObject (Variables|/Game/Level/Blueprints/BP_cube.BP_cube_C|GetCube1 _asbp_cube)))
          (:CastFailed
            (bind _asbp_pan (Utilities|Casting|CastToBP_pan (.HitActor (Collision|BreakHitResult _outhit)))
              (:then
                (Variables|/Game/Level/Blueprints/BP_pan.BP_pan_C|SetdiatasKompor _asbp_pan false)
                (CallFunction|GrabPan _asbp_pan))
              (:CastFailed
                (bind _asbp_egg (Utilities|Casting|CastToBP_egg (.HitActor (Collision|BreakHitResult _outhit)))
                  (:then
                    (Variables|/Game/Level/Blueprints/BP_egg.BP_egg_C|Setgrabbed _asbp_egg true)
                    (CallFunction|MoveObject (Variables|/Game/Level/Blueprints/BP_egg.BP_egg_C|Getegg _asbp_egg) _asbp_egg))
                  (:CastFailed
                    (bind _asbp_knob_kompor (Utilities|Casting|CastToBP_knobKompor (.HitActor (Collision|BreakHitResult _outhit)))
                      (:then
                        (Default|Togglekompordariknob _asbp_knob_kompor))
                      (:CastFailed
                        (Utilities|Casting|CastTobp_eggRack (.HitActor (Collision|BreakHitResult _outhit))
                          (:then
                            (bind _returnvalue_4 (Game|SpawnActorfromClass "/Game/Level/Blueprints/BP_egg.BP_egg_C" _returnvalue "Undefined" 0 0))
                            (Variables|/Game/Level/Blueprints/BP_egg.BP_egg_C|Setgrabbed _returnvalue_4 true)
                            (Collision|SetCollisionObjectType (Variables|/Game/Level/Blueprints/BP_egg.BP_egg_C|Getegg _returnvalue_4) "ECC_Pawn")
                            (CallFunction|MoveObject (Variables|/Game/Level/Blueprints/BP_egg.BP_egg_C|Getegg _returnvalue_4) _returnvalue_4))
                          (:CastFailed
                            (Utilities|Casting|CastToBP_panRack (.HitActor (Collision|BreakHitResult _outhit))
                              (:then
                                (bind _returnvalue_5 (Game|SpawnActorfromClass "/Game/Level/Blueprints/BP_pan.BP_pan_C" _returnvalue "Undefined" 0 0))
                                (CallFunction|GrabPan _returnvalue_5))
                              (:CastFailed
                                (bind _asbp_piring (Utilities|Casting|CastToBP_piring (.HitActor (Collision|BreakHitResult _outhit)))
                                  (:then
                                    (CallFunction|MoveObject (Variables|/Game/Level/Blueprints/BP_piring.BP_piring_C|GetPlate _asbp_piring)))
                                  (:CastFailed
                                    (Utilities|Casting|CastToBP_plateRack (.HitActor (Collision|BreakHitResult _outhit)))
                                    (bind _returnvalue_6 (Game|SpawnActorfromClass "/Game/Level/Blueprints/BP_piring.BP_piring_C" _returnvalue "Undefined" 0 0))
                                    (CallFunction|MoveObject (Variables|/Game/Level/Blueprints/BP_piring.BP_piring_C|GetPlate _returnvalue_6))))))))))))))))))))

(event OnHandReleased(Leap)
  (params (Hand :type Leap%20Hand%20Data%20Structure%20%28by%20ref%29))
  (Variables|Default|Setgrabbed false))

(event OnHandEndTracking(Leap)
  (params (Hand :type Leap%20Hand%20Data%20Structure%20%28by%20ref%29))
  (Transformation|SetWorldLocation (Variables|Default|GetSkeletalMesh) "0.000000,0.000000,1000000000.000000" false false)
  (Development|PrintString "Hello"))

(event Custom|moveObject
  (params (targetObject :type Static%20Mesh%20Component%20Object%20Reference) (targetActor :type Actor%20Object%20Reference))
  (Utilities|IsValid targetObject :!label _label
    (:Is%20Valid
      (if (Variables|Default|Getgrabbed)
        (Physics|SetSimulatePhysics targetObject false)
        (Transformation|SetWorldLocation targetObject (Variables|Default|GetHand%20Pos) false false)
        (Physics|SetEnableGravity targetObject false)
        (Utilities|FlowControl|Delay 0.001)
        (goto _label)
        (else
          (Physics|SetSimulatePhysics targetObject true)
          (Physics|SetEnableGravity targetObject true)
          (Utilities|IsValid targetActor
            (:Is%20Valid
              (bind _asbp_egg (Utilities|Casting|CastToBP_egg targetActor))
              (Variables|/Game/Level/Blueprints/BP_egg.BP_egg_C|Setgrabbed _asbp_egg false))))))))

(event Custom|grab%20pan
  (params (pan :type BP%20Pan%20Object%20Reference))
  (bind _hand (Variables|Default|Gethand))
  (bind (_arm _confidence _digits _flags _grabangle _grabstrength _handtype _index _middle _palm) (Utilities|Struct|BreakLeapHandData _hand))
  (Utilities|IsValid pan :!label _label
    (:Is%20Valid
      (if (Variables|Default|Getgrabbed)
        (Physics|SetEnableGravity (Variables|/Game/Level/Blueprints/BP_pan.BP_pan_C|Getpan pan) false)
        (Physics|SetSimulatePhysics (Variables|/Game/Level/Blueprints/BP_pan.BP_pan_C|Getpan pan) false)
        (Transformation|SetWorldLocationAndRotation (Variables|/Game/Level/Blueprints/BP_pan.BP_pan_C|Getpan pan) (+ (Variables|Default|GetHand%20Pos) "0.000000,-60.000000,0.000000") (Math|Rotator|MakeRotator (* (* (+ (.pitch (.Orientation (Utilities|Struct|BreakLeapPalmData _palm))) -75.0) 3.0) -1.0) (* (+ (.roll (.Rotation (Utilities|Struct|BreakLeapBoneData _arm))) -45.0) -1.0) 9e+01) false false)
        (Utilities|FlowControl|Delay 0.01)
        (goto _label)
        (else
          (Physics|SetSimulatePhysics (Variables|/Game/Level/Blueprints/BP_pan.BP_pan_C|Getpan pan) true)
          (Physics|SetEnableGravity (Variables|/Game/Level/Blueprints/BP_pan.BP_pan_C|Getpan pan) true))))))

(event EventBeginPlay
  (bind _asbp_player (Utilities|Casting|CastToBP_player (Game|GetPlayerCharacter 0)))
  (Variables|Default|SetAs%20BP%20Player _asbp_player))

(event Collision|EventActorBeginOverlap
  (params (OtherActor :type Actor%20Object%20Reference)))

(event EventTick
  (params (DeltaSeconds :type Float%20%28single-precision%29)))

(fn ConstructionScript)

(fn SetLeftanim
  (params (Lefthand :type Leap%20Hand%20Data%20Structure))
  (bind _asleap_low_poly_left_stretch_anim_bp (Utilities|Casting|CastToLeapLowPolyLeftStretchAnimBP (Components|SkeletalMesh|GetAnimInstance (Variables|Default|GetSkeletalMesh))))
  (Default|SetAnimData _asleap_low_poly_left_stretch_anim_bp Lefthand))