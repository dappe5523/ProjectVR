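; BP_Yolk is an egg actor that can sit in a pan and cook.
; Box overlap starts a self-repeating check that sphere-traces around White, caches any BP_pan hit and snaps White to its location.
; End overlap also sets InPan true, so leaving never clears the flag.
; The memasak (cook) event accumulates heat into Doneness, printing it or "hangus" (burnt) past the limit.
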(event OnComponentBeginOverlap(Box)
  (params (OverlappedComponent :type Primitive%20Component%20Object%20Reference) (OtherActor :type Actor%20Object%20Reference) (OtherComp :type Primitive%20Component%20Object%20Reference) (OtherBodyIndex :type Integer) (bFromSweep :type Boolean) (SweepResult :type Hit%20Result%20Structure%20%28by%20ref%29))
  (Variables|Default|SetinPan true)
  (CallFunction|IsinPan))

(event OnComponentEndOverlap(Box)
  (params (OverlappedComponent :type Primitive%20Component%20Object%20Reference) (OtherActor :type Actor%20Object%20Reference) (OtherComp :type Primitive%20Component%20Object%20Reference) (OtherBodyIndex :type Integer))
  (Variables|Default|SetinPan true))

(event Custom|memasak
  (params (heat :type Float%20%28double-precision%29))
  (bind _output_get (Variables|Default|Setdoneness (+ (Variables|Default|Getdoneness) heat)))
  (if (> _output_get 1e+02)
    (Development|PrintString "hangus")
    (else
      (Development|PrintString (Utilities|String|ToString(Float) _output_get) true true "(R=0.000000,G=0.660000,B=1.000000,A=1.000000)" _output_get))))

(event Custom|isInPan
  (bind _white (Variables|Default|GetWhite))
  (bind _returnvalue (Transformation|GetWorldLocation _white))
  (if (Variables|Default|GetinPan)
    (bind (_outhit _returnvalue_2) (Collision|SphereTraceForObjects _returnvalue _returnvalue 5e+02 (Variables|Default|GetObject%20Types) false 0 "None"))
    (if _returnvalue_2
      (bind _asbp_pan (Utilities|Casting|CastToBP_pan (.HitActor (Collision|BreakHitResult _outhit))))
      (Variables|Default|Setpan _asbp_pan)
      (Transformation|SetWorldLocation (Variables|Default|GetWhite) (Transformation|GetActorLocation _asbp_pan) false false)
      (Utilities|FlowControl|Delay 0.01)
      (CallFunction|IsinPan))))

(event EventBeginPlay)

(event Collision|EventActorBeginOverlap
  (params (OtherActor :type Actor%20Object%20Reference)))

(event EventTick
  (params (DeltaSeconds :type Float%20%28single-precision%29)))

(fn ConstructionScript)