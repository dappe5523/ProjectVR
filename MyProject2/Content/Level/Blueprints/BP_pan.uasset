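; Frying pan actor for a cooking game that takes in eggs and tracks how cooked they are.
; While something is in InputBox, a 0.1-second loop sphere-traces for ungrabbed BP_egg actors, stores their food value, destroys them and shows a fried-egg mesh.
; The cook event adds heat to the first food entry, updates the cook-bar widget created on first grab, and toggles sound.
; A separate empty event only hides the egg mesh.
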(event OnComponentBeginOverlap(inputbox)
  (params (OverlappedComponent :type Primitive%20Component%20Object%20Reference) (OtherActor :type Actor%20Object%20Reference) (OtherComp :type Primitive%20Component%20Object%20Reference) (OtherBodyIndex :type Integer) (bFromSweep :type Boolean) (SweepResult :type Hit%20Result%20Structure%20%28by%20ref%29))
  (Variables|Default|SetinRadius true)
  (Components|Activation|Activate (Variables|Default|Getinput%20box) false))

(event OnComponentActivated(inputbox)
  (params (Component :type Actor%20Component%20Object%20Reference) (bReset :type Boolean))
  (CallFunction|Activate :!label _label)
  (Utilities|FlowControl|Delay 0.1)
  (if (Variables|Default|GetinRadius)
    (goto _label)))

(event OnComponentEndOverlap(inputbox)
  (params (OverlappedComponent :type Primitive%20Component%20Object%20Reference) (OtherActor :type Actor%20Object%20Reference) (OtherComp :type Primitive%20Component%20Object%20Reference) (OtherBodyIndex :type Integer))
  (Variables|Default|SetinRadius false)
  (Components|Activation|Deactivate (Variables|Default|Getinput%20box)))

(event Custom|activate
  (bind _actors_to_ignore_0 (Variables|Default|GetActors%20to%20Ignore_0))
  (bind _pan (Variables|Default|Getpan))
  (bind _returnvalue (Transformation|GetWorldLocation _pan))
  (bind _outhit (Collision|SphereTraceForObjects _returnvalue _returnvalue 1e+02 (Variables|Default|GetObject%20Types) false _actors_to_ignore_0 "ForOneFrame"))
  (Utilities|IsValid (.HitActor (Collision|BreakHitResult _outhit))
    (:Is%20Valid
      (bind _asbp_egg (Utilities|Casting|CastToBP_egg (.HitActor (Collision|BreakHitResult _outhit)))
        (:then
          (if (not (Variables|/Game/Level/Blueprints/BP_egg.BP_egg_C|Getgrabbed _asbp_egg))
            (Utilities|Array|Add (Variables|Default|Getfoodvalue) (Variables|/Game/Level/Blueprints/BP_egg.BP_egg_C|Getfoodvalue _asbp_egg))
            (if (== (.foodtype (Utilities|Struct|Breakstrruct_food (Variables|/Game/Level/Blueprints/BP_egg.BP_egg_C|Getfoodvalue _asbp_egg))) "egg")
              (Rendering|SetVisibility (Variables|Default|Getsunny%20side%20up%20egg) true true)
              (Actor|DestroyActor _asbp_egg)
              (Variables|Default|Setadakonten true))))
        (:CastFailed
          (Utilities|Array|Add _actors_to_ignore_0 (.HitActor (Collision|BreakHitResult _outhit))))))))

(event Custom|empty
  (Rendering|SetVisibility (Variables|Default|Getsunny%20side%20up%20egg) false true))

(event Custom|grabbed
  (if (not (Variables|Default|Getconditionwg))
    (Variables|Default|Setconditionwg true)
    (bind _returnvalue (UserInterface|CreateWidget "/Game/Level/UI/wg_cookbar.wg_cookbar_C"))
    (Variables|Default|Setwg_bar _returnvalue)
    (UserInterface|SetWidget (Variables|Default|GetWidget) _returnvalue)))

(event Custom|cook
  (params (heat :type Float%20%28double-precision%29))
  (bind _foodvalue (Variables|Default|Getfoodvalue))
  (bind _foodvalue_2 (Variables|Default|Getfoodvalue))
  (bind _output (Utilities|Array|Get(acopy) _foodvalue))
  (bind _output_2 (Utilities|Array|Get(acopy) _foodvalue_2))
  (bind _cookvalue (Utilities|Struct|Breakstrruct_food _output))
  (Variables|Default|Setcooking true)
  (CallFunction|Togglesound)
  (if (> (Utilities|Array|Length _foodvalue_2) 0)
    (Development|PrintString "aa")
    (Utilities|Array|SetArrayElem _foodvalue_2 0 (Utilities|Struct|Makestrruct_food (+ (.cookvalue _output_2) heat) (.foodtype _output_2)))
    (Development|PrintString (Utilities|String|ToString(Float) _cookvalue))
    (Default|Update (Variables|Default|Getwg_bar) (/ _cookvalue 1e+02))))

(event Custom|togglesound
  (bind _soundeffect (Variables|Default|GetSoundEffect))
  (if (Variables|Default|GetisOnmusic)
    (if (not (Variables|Default|Getcooking))
      (Class|AudioLinkBlueprintInterface|StopLink(Message) _soundeffect)
      (Variables|Default|SetisOnmusic false))
    (else
      (Audio|PlaySound2D _soundeffect 1.0 1.0 0.0 0 0)
      (Variables|Default|SetisOnmusic true))))

(event EventBeginPlay)

(event Collision|EventActorBeginOverlap
  (params (OtherActor :type Actor%20Object%20Reference)))

(event EventTick
  (params (DeltaSeconds :type Float%20%28single-precision%29))
  (bind _pan (Variables|Default|Getpan))
  (if (Variables|Default|GetdiatasKompor)
    (Collision|SetCollisionObjectType _pan "ECC_Pawn")
    (else
      (Collision|SetCollisionObjectType _pan "ECC_Pawn"))))

(fn ConstructionScript)