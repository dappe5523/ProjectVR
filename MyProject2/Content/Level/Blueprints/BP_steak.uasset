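; BP_steak is a two-sided cookable steak that tracks doneness for each side as heat is applied.
; Each tick, a short line trace near the Atas component sets which side receives heat, while the widget repositions above the steak and turns toward the player.
; The cook event adds heat to that side, then writes the two-side average to the progress bar and Foodvalue.
; The first grab creates the bar and starts a sizzle sound, which togglesound controls.
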(event Custom|cook
  (params (heat :type Float%20%28double-precision%29))
  (bind _bar (Variables|Default|Getbar))
  (if (Variables|Default|Gettop?)
    (bind _output_get (Variables|Default|SetdonenessAtas (+ (Variables|Default|GetdonenessAtas) heat)))
    (Development|PrintString (Utilities|String|ToString(Float) _output_get))
    (Utilities|IsValid _bar
      (:Is%20Valid
        _))
    (else
      (bind _output_get_2 (Variables|Default|SetdonenessBawah (+ (Variables|Default|GetdonenessBawah) heat)))
      (Development|PrintString (Utilities|String|ToString(Float) _output_get_2))))
  (Default|Update _bar (/ (/ (+ _output_get _output_get_2) 2.0) 1e+02))
  (Variables|Default|Setfoodvalue (Utilities|Struct|Makestrruct_food (/ (+ _output_get _output_get_2) 2.0) "steak")))

(event Custom|grabbed
  (if (Variables|Default|GetCondition)
    (bind _returnvalue (Audio|SpawnSound2D "/Game/Level/sound_and_music/cooking-steak-23404.cooking-steak-23404" 1.0 1.0 0.0 0 false false))
    (Variables|Default|SetsoundEffect _returnvalue)
    (Variables|Default|SetCondition false)
    (bind _returnvalue_2 (UserInterface|CreateWidget "/Game/Level/UI/wg_cookbar.wg_cookbar_C"))
    (Variables|Default|Setbar _returnvalue_2)
    (UserInterface|SetWidget (Variables|Default|GetWidget) _returnvalue_2)))

(event Custom|togglesound
  (params (on/off :type Boolean))
  (if (Variables|Default|GetismusicOn)
    (Utilities|IsValid (Variables|Default|GetsoundEffect)
      (:Is%20Valid
        (Utilities|FlowControl|Delay 1e+01)
        (Components|DestroyComponent (Variables|Default|GetsoundEffect)))
      (:Is%20Not%20Valid
        (Variables|Default|SetismusicOn false)))
    (else
      (bind _returnvalue (Audio|SpawnSound2D "/Game/Level/sound_and_music/cooking-steak-23404.cooking-steak-23404" 1.0 1.0 0.0 0))
      (Variables|Default|SetsoundEffect _returnvalue)
      (Variables|Default|SetismusicOn true))))

(event EventBeginPlay
  (Input|EnableInput (Game|GetPlayerController 0)))

(event Collision|EventActorBeginOverlap
  (params (OtherActor :type Actor%20Object%20Reference)))

(event EventTick
  (params (DeltaSeconds :type Float%20%28single-precision%29))
  (bind _widget (Variables|Default|GetWidget))
  (bind _actors_to_ignore (Variables|Default|GetActors%20to%20Ignore))
  (bind _atas (Variables|Default|Getatas))
  (bind _returnvalue (Transformation|GetWorldLocation _atas))
  (Transformation|SetWorldRotation (Variables|Default|GetWidget) (Math|Conversions|RotationFromXVector (Math|Vector|RotateVector (Math|Vector|Normalize (* (- (Transformation|GetActorLocation (Game|GetPlayerCharacter 0)) (Transformation|GetWorldLocation (Variables|Default|GetWidget))) "1.000000,1.000000,0.000000")) "0, 0, 0")) false false)
  (bind _outhit (Collision|LineTraceForObjects (+ _returnvalue "0.000000,0.000000,10.000000") (+ _returnvalue "0.000000,0.000000,5.000000") (Variables|Default|GetObject%20Types) false _actors_to_ignore "ForOneFrame" false))
  (Utilities|Casting|CastToBP_steak (.HitActor (Collision|BreakHitResult _outhit))
    (:then
      (if (== (.HitComponent (Collision|BreakHitResult _outhit)) (Variables|Default|Getatas))
        (Variables|Default|Settop? false)
        (Transformation|SetWorldLocation _widget (+ (Transformation|GetWorldLocation (Variables|Default|Getatas)) "0.000000,0.000000,30.000000") false false)
        (elif (== (.HitComponent (Collision|BreakHitResult _outhit)) (Variables|Default|Getbawah))
          (Variables|Default|Settop? true)
          (Transformation|SetWorldLocation _widget (+ (Transformation|GetWorldLocation (Variables|Default|Getbawah)) "0.000000,0.000000,30.000000") false false))))
    (:CastFailed
      (Utilities|Array|Add _actors_to_ignore (.HitActor (Collision|BreakHitResult _outhit))))))

(event Input|KeyboardEvents|B
  (params (Key :type Key%20Structure :default "None")))

(fn ConstructionScript)