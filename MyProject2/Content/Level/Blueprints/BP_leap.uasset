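; BP_leap is a Leap Motion hand controller that lets the player grab and carry cube and pan objects.
; Each tracking frame picks a left or right palm, converts its axes with a scale multiplier and moves the skeletal mesh to it.
; A grab sphere-traces at the mesh for BP_cube or BP_pan, then a short Delay loop pins the hit part to the palm with gravity off until release restores it.
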(event OnHandGrabbed(Leap)
  (params (Hand :type Leap%20Hand%20Data%20Structure%20%28by%20ref%29))
  (bind _multiply (Variables|Default|Getmultiply))
  (bind _selecthand (Variables|Default|GetSelectHand))
  (bind _skeletalmesh (Variables|Default|GetSkeletalMesh))
  (bind (_direction _normal _orientation _position) (Utilities|Struct|BreakLeapPalmData _selecthand))
  (bind _returnvalue (Transformation|GetWorldLocation _skeletalmesh))
  (bind _returnvalue_2 (* (.y _position) -1.0))
  (bind _returnvalue_3 (* (Math|Vector|MakeVector (.z _position) _returnvalue_2 (.x _position)) _multiply))
  (Variables|Default|Setgrabbed true)
  (bind (_outhit _returnvalue_4) (Collision|SphereTraceForObjects _returnvalue (+ _returnvalue "") 1e+02 (Variables|Default|GetObject%20Types) false 0 "ForDuration"))
  (if _returnvalue_4
    (bind _asbp_cube (Utilities|Casting|CastToBP_cube (.HitActor (Collision|BreakHitResult _outhit)))
      (:then
        (if (Variables|Default|Getgrabbed) :!label _label
          (Transformation|SetWorldLocation (Variables|/Game/Level/Blueprints/BP_cube.BP_cube_C|GetCube1 _asbp_cube) _returnvalue_3 false false)
          (Physics|SetEnableGravity (Variables|/Game/Level/Blueprints/BP_cube.BP_cube_C|GetCube1 _asbp_cube) false)
          (Utilities|FlowControl|Delay 0.001)
          (goto _label)
          (else
            (Physics|SetEnableGravity (Variables|/Game/Level/Blueprints/BP_cube.BP_cube_C|GetCube1 _asbp_cube) true))))
      (:CastFailed
        (bind _asbp_pan (Utilities|Casting|CastToBP_pan (.HitActor (Collision|BreakHitResult _outhit))))
        (if (Variables|Default|Getgrabbed) :!label _label_2
          (Transformation|SetWorldLocation (Variables|/Game/Level/Blueprints/BP_pan.BP_pan_C|Gethead _asbp_pan) _returnvalue_3 false false)
          (Physics|SetEnableGravity (Variables|/Game/Level/Blueprints/BP_pan.BP_pan_C|Gethead _asbp_pan) false)
          (Utilities|FlowControl|Delay 0.001)
          (goto _label_2)
          (else
            (Physics|SetEnableGravity (Variables|/Game/Level/Blueprints/BP_pan.BP_pan_C|Gethead _asbp_pan) true)))))))

(event OnLeapTrackingData(Leap)
  (params (Frame :type Leap%20Frame%20Data%20Structure%20%28by%20ref%29))
  (for _array_element (.Hands (Utilities|Struct|BreakLeapFrameData Frame))
    (switch Utilities|FlowControl|Switch|SwitchonEHandType (.HandType (Utilities|Struct|BreakLeapHandData _array_element))
      (:LEAP_HAND_LEFT
        (Variables|Default|SetLeft _array_element)
        (Variables|Default|SetisRigthHandActive false))
      (:LEAP_HAND_RIGHT
        (Variables|Default|SetRIght _array_element)
        (Variables|Default|SetisRigthHandActive true))))
  (if (Variables|Default|GetisRigthHandActive)
    (Variables|Default|SetSelectHand (.Palm (Utilities|Struct|BreakLeapHandData (Variables|Default|GetRIght))))
    (else
      (Variables|Default|SetSelectHand (.Palm (Utilities|Struct|BreakLeapHandData (Variables|Default|GetLeft))))))
  (Transformation|SetWorldLocationAndRotation (Variables|Default|GetSkeletalMesh) (* (Math|Vector|MakeVector (.z (.Position (Utilities|Struct|BreakLeapPalmData (Variables|Default|GetSelectHand)))) (* (.y (.Position (Utilities|Struct|BreakLeapPalmData (Variables|Default|GetSelectHand)))) -1.0) (.x (.Position (Utilities|Struct|BreakLeapPalmData (Variables|Default|GetSelectHand))))) (Variables|Default|Getmultiply)) (.Orientation (Utilities|Struct|BreakLeapPalmData (Variables|Default|GetSelectHand))) false false))

(event OnHandReleased(Leap)
  (params (Hand :type Leap%20Hand%20Data%20Structure%20%28by%20ref%29))
  (Variables|Default|Setgrabbed false))

(event EventBeginPlay)

(event Collision|EventActorBeginOverlap
  (params (OtherActor :type Actor%20Object%20Reference)))

(event EventTick
  (params (DeltaSeconds :type Float%20%28single-precision%29)))

(fn ConstructionScript)