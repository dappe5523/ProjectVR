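; BP_pan2 is a pan actor that accepts a single BP_egg2 and shows it as its contents.
; A sphere overlap triggers a debug-drawn sphere trace at the pan's location; a found egg is destroyed, the Egg component is revealed and AdaKonten blocks further eggs.
; Non-egg hits join a never-cleared ignore list, and the trace repeats after a short delay, with Indonesian debug prints reporting each outcome.
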(event OnComponentBeginOverlap(Sphere)
  (params (OverlappedComponent :type Primitive%20Component%20Object%20Reference) (OtherActor :type Actor%20Object%20Reference) (OtherComp :type Primitive%20Component%20Object%20Reference) (OtherBodyIndex :type Integer) (bFromSweep :type Boolean) (SweepResult :type Hit%20Result%20Structure%20%28by%20ref%29))
  (bind _returnvalue (Transformation|GetActorLocation))
  (bind (_outhit _returnvalue_2) (Collision|SphereTraceForObjects _returnvalue _returnvalue 5e+01 (Variables|Default|GetObject%20Types) false (Variables|Default|GetActors%20to%20Ignore_0) "ForDuration" :!label _label))
  (if _returnvalue_2
    (Utilities|IsValid (.HitActor (Collision|BreakHitResult _outhit))
      (:Is%20Valid
        (bind _asbp_egg_2 (Utilities|Casting|CastToBP_egg2 (.HitActor (Collision|BreakHitResult _outhit)))
          (:then
            (if (Variables|Default|GetadaKonten)
              (Development|PrintString "sudah ada")
              (else
                (Actor|DestroyActor _asbp_egg_2)
                (Rendering|SetVisibility (Variables|Default|Getegg) true true)
                (Development|PrintString "telur masuk")
                (Variables|Default|Setadakonten true))))
          (:CastFailed
            (Utilities|Array|Add (Variables|Default|GetActors%20to%20Ignore_0) (.HitActor (Collision|BreakHitResult _outhit)))
            (Utilities|FlowControl|Delay 0.2)
            (Development|PrintString "bukan telur masuk")
            (goto _label)))))))

(event EventBeginPlay)

(event Collision|EventActorBeginOverlap
  (params (OtherActor :type Actor%20Object%20Reference)))

(event EventTick
  (params (DeltaSeconds :type Float%20%28single-precision%29)))

(fn ConstructionScript)