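; BP_tong is a tong actor that flips a BP_steak when its Box collision overlaps one.
; On overlap, it adds 180 degrees of roll to the steak's Atas component in world space and clears a Condition flag to block repeat flips.
; When any overlap with the box ends, a one-second delay re-arms the flag, acting as a simple flip cooldown.
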(event OnComponentBeginOverlap(Box)
  (params (OverlappedComponent :type Primitive%20Component%20Object%20Reference) (OtherActor :type Actor%20Object%20Reference) (OtherComp :type Primitive%20Component%20Object%20Reference) (OtherBodyIndex :type Integer) (bFromSweep :type Boolean) (SweepResult :type Hit%20Result%20Structure%20%28by%20ref%29))
  (bind _asbp_steak (Utilities|Casting|CastToBP_steak OtherActor))
  (if (Variables|Default|GetCondition)
    (Variables|Default|SetCondition false)
    (Transformation|SetWorldRotation (Variables|/Game/Level/Blueprints/BP_steak.BP_steak_C|Getatas _asbp_steak) (Math|Rotator|MakeRotator (+ (.roll (Transformation|GetWorldRotation (Variables|/Game/Level/Blueprints/BP_steak.BP_steak_C|Getatas _asbp_steak))) 1.8e+02) (.pitch (Transformation|GetWorldRotation (Variables|/Game/Level/Blueprints/BP_steak.BP_steak_C|Getatas _asbp_steak))) (.yaw (Transformation|GetWorldRotation (Variables|/Game/Level/Blueprints/BP_steak.BP_steak_C|Getatas _asbp_steak)))) false false)))

(event OnComponentEndOverlap(Box)
  (params (OverlappedComponent :type Primitive%20Component%20Object%20Reference) (OtherActor :type Actor%20Object%20Reference) (OtherComp :type Primitive%20Component%20Object%20Reference) (OtherBodyIndex :type Integer))
  (Utilities|FlowControl|Delay 1.0)
  (Variables|Default|SetCondition true))

(event EventBeginPlay)

(event Collision|EventActorBeginOverlap
  (params (OtherActor :type Actor%20Object%20Reference)))

(event EventTick
  (params (DeltaSeconds :type Float%20%28single-precision%29)))

(fn ConstructionScript)