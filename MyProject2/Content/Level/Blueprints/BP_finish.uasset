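; BP_finish is a level goal zone that checks whether a plate (BP_piring) holds the required dish and triggers the player's win.
; While its box is overlapped, it repeats a sphere trace every 0.1 seconds, ignoring non-plate hits until nothing is found.
; Plate food must match GoalFood in count, with each goal type present at sufficient Cookvalue.
; Win receives an over-200 Cookvalue flag that reflects only the last food item.
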(event OnComponentBeginOverlap(Box)
  (params (OverlappedComponent :type Primitive%20Component%20Object%20Reference) (OtherActor :type Actor%20Object%20Reference) (OtherComp :type Primitive%20Component%20Object%20Reference) (OtherBodyIndex :type Integer) (bFromSweep :type Boolean) (SweepResult :type Hit%20Result%20Structure%20%28by%20ref%29))
  (Variables|Default|Setisactive true)
  (if (Variables|Default|Getisactive) :!label _label
    (CallFunction|Active)
    (Utilities|FlowControl|Delay 0.1)
    (goto _label)))

(event OnComponentEndOverlap(Box)
  (params (OverlappedComponent :type Primitive%20Component%20Object%20Reference) (OtherActor :type Actor%20Object%20Reference) (OtherComp :type Primitive%20Component%20Object%20Reference) (OtherBodyIndex :type Integer))
  (Variables|Default|Setisactive false))

(event Custom|active
  (bind _returnvalue (Transformation|GetActorLocation))
  (bind _goalfood (Variables|Default|GetgoalFood))
  (bind (_outhit _returnvalue_2) (Collision|SphereTraceForObjects _returnvalue _returnvalue 1e+02 (Variables|Default|GetObject%20Types) false (Variables|Default|GetActors%20to%20Ignore) "ForDuration"))
  (if _returnvalue_2
    (bind _asbp_piring (Utilities|Casting|CastToBP_piring (.HitActor (Collision|BreakHitResult _outhit)))
      (:then
        (if (== (Utilities|Array|Length _goalfood) (Utilities|Array|Length (Variables|/Game/Level/Blueprints/BP_piring.BP_piring_C|Getfood _asbp_piring)))
          (bind _array_element (Utilities|Array|ForEachLoopwithBreak _goalfood)
            (:LoopBody
              (bind _array_element_2 (Utilities|Array|ForEachLoopwithBreak (Variables|/Game/Level/Blueprints/BP_piring.BP_piring_C|Getfood _asbp_piring))
                (:LoopBody
                  (if (== (.foodtype (Utilities|Struct|Breakstrruct_food _array_element)) (.foodtype (Utilities|Struct|Breakstrruct_food _array_element_2)))
                    (if (>= (.cookvalue (Utilities|Struct|Breakstrruct_food _array_element_2)) (.cookvalue (Utilities|Struct|Breakstrruct_food _array_element)))
                      (Variables|Default|Setiscorrect true))))
                (:Completed
                  (if (Variables|Default|Getiscorrect)
                    (Variables|Default|Setiscorrect false)
                    (else
                      (Variables|Default|Setfoodiscorrect false))))))
            (:Completed
              (if (Variables|Default|Getfoodiscorrect)
                (Development|PrintString "menang")
                (bind _asbp_player (Utilities|Casting|CastToBP_player (Game|GetPlayerCharacter 0)))
                (for _array_element_3 (Variables|/Game/Level/Blueprints/BP_piring.BP_piring_C|Getfood _asbp_piring)
                  (Variables|Default|SetNewVar (> (.cookvalue (Utilities|Struct|Breakstrruct_food _array_element_3)) 2e+02)))
                (Default|Win _asbp_player (Variables|Default|GetNewVar))
                (else
                  (Variables|Default|Setfoodiscorrect true)
                  (Development|PrintString "tidak benar")))))))
      (:CastFailed
        (Utilities|Array|Add (Variables|Default|GetActors%20to%20Ignore) 0)))
    (else
      (Variables|Default|Setisactive false)
      (Variables|Default|SetActors%20to%20Ignore (Variables|Default|Getempty)))))

(event EventBeginPlay)

(event Collision|EventActorBeginOverlap
  (params (OtherActor :type Actor%20Object%20Reference)))

(event EventTick
  (params (DeltaSeconds :type Float%20%28single-precision%29)))

(fn ConstructionScript)