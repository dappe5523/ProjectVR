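; Player Blueprint that rotates its Camera in response to overlaps and key presses.
; Kiri and Kanan volumes start 0.01-second Delay loops that step yaw down or up while touched by BP_leapKiri or BP_leapkanan, respectively.
; Both loops share one On flag, set before the cast on any overlap and cleared when the matching actor exits.
; W and S snap pitch up or down 45 degrees, zeroing yaw and roll.
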(event OnComponentBeginOverlap(kiri)
  (params (OverlappedComponent :type Primitive%20Component%20Object%20Reference) (OtherActor :type Actor%20Object%20Reference) (OtherComp :type Primitive%20Component%20Object%20Reference) (OtherBodyIndex :type Integer) (bFromSweep :type Boolean) (SweepResult :type Hit%20Result%20Structure%20%28by%20ref%29))
  (bind _camera (Variables|Default|GetCamera))
  (bind _returnvalue (Transformation|GetWorldRotation _camera))
  (Variables|Default|Seton? true)
  (Utilities|Casting|CastToBP_leapKiri OtherActor)
  (Utilities|FlowControl|Delay 0.01 :!label _label)
  (if (Variables|Default|Geton?)
    (Transformation|SetWorldRotation (Variables|Default|GetCamera) (Math|Rotator|MakeRotator (.roll _returnvalue) (.pitch _returnvalue) (- (.yaw _returnvalue) 1.0)) false false)
    (goto _label)))

(event OnComponentEndOverlap(kiri)
  (params (OverlappedComponent :type Primitive%20Component%20Object%20Reference) (OtherActor :type Actor%20Object%20Reference) (OtherComp :type Primitive%20Component%20Object%20Reference) (OtherBodyIndex :type Integer))
  (Utilities|Casting|CastToBP_leapKiri OtherActor)
  (Variables|Default|Seton? false))

(event OnComponentBeginOverlap(kanan)
  (params (OverlappedComponent :type Primitive%20Component%20Object%20Reference) (OtherActor :type Actor%20Object%20Reference) (OtherComp :type Primitive%20Component%20Object%20Reference) (OtherBodyIndex :type Integer) (bFromSweep :type Boolean) (SweepResult :type Hit%20Result%20Structure%20%28by%20ref%29))
  (bind _camera (Variables|Default|GetCamera))
  (bind _returnvalue (Transformation|GetWorldRotation _camera))
  (Variables|Default|Seton? true)
  (Utilities|Casting|CastToBP_leapkanan OtherActor)
  (Utilities|FlowControl|Delay 0.01 :!label _label)
  (if (Variables|Default|Geton?)
    (Transformation|SetWorldRotation _camera (Math|Rotator|MakeRotator (.roll _returnvalue) (.pitch _returnvalue) (+ (.yaw _returnvalue) 1.0)) false false)
    (goto _label)))

(event OnComponentEndOverlap(kanan)
  (params (OverlappedComponent :type Primitive%20Component%20Object%20Reference) (OtherActor :type Actor%20Object%20Reference) (OtherComp :type Primitive%20Component%20Object%20Reference) (OtherBodyIndex :type Integer))
  (Utilities|Casting|CastToBP_leapkanan OtherActor)
  (Variables|Default|Seton? false))

(event EventBeginPlay)

(event Collision|EventActorBeginOverlap
  (params (OtherActor :type Actor%20Object%20Reference)))

(event EventTick
  (params (DeltaSeconds :type Float%20%28single-precision%29)))

(event Input|KeyboardEvents|W
  (params (Key :type Key%20Structure))
  (:Pressed
    (Transformation|SetWorldRotation (Variables|Default|GetCamera) (Math|Rotator|MakeRotator 0.0 (+ 0.0 45.0) 0.0) false false)))

(event Input|KeyboardEvents|S
  (params (Key :type Key%20Structure))
  (:Pressed
    (Transformation|SetWorldRotation (Variables|Default|GetCamera) (Math|Rotator|MakeRotator 0.0 (- 0.0 45.0) 0.0) false false)))

(fn ConstructionScript)