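; BP_kompor is a stove that cooks pans and steaks placed on it, with a Grill flag that skips pan snapping.
; Overlapping its box starts a repeating Delay loop that sphere-traces for the item, snaps pans in place and calls Cook with the heat level while on.
; togglekompor cycles heat through off and three levels, updating its display and the pan's on-stove flag.
; Tick feeds the pan's first food cook value to a widget progress bar.
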(event OnComponentBeginOverlap(Box)
  (params (OverlappedComponent :type Primitive%20Component%20Object%20Reference) (OtherActor :type Actor%20Object%20Reference) (OtherComp :type Primitive%20Component%20Object%20Reference) (OtherBodyIndex :type Integer) (bFromSweep :type Boolean) (SweepResult :type Hit%20Result%20Structure%20%28by%20ref%29))
  (Components|Activation|Activate (Variables|Default|GetBox) false))

(event OnComponentActivated(Box)
  (params (Component :type Actor%20Component%20Object%20Reference) (bReset :type Boolean))
  (CallFunction|Active :!label _label)
  (Utilities|FlowControl|Delay 0.1)
  (goto _label))

(event OnComponentEndOverlap(Box)
  (params (OverlappedComponent :type Primitive%20Component%20Object%20Reference) (OtherActor :type Actor%20Object%20Reference) (OtherComp :type Primitive%20Component%20Object%20Reference) (OtherBodyIndex :type Integer))
  (Components|Activation|Deactivate (Variables|Default|GetBox)))

(event Custom|togglekompor
  (bind _heatlevelwg (Variables|Default|GetHeatLevelWG))
  (bind _onkompor (Variables|Default|GetonKompor))
  (if (== (Variables|Default|Getheat%20level) 0)
    (Variables|Default|Setheat%20level 1)
    (Default|Change _heatlevelwg (Variables|Default|Getheat%20level) :!label _label)
    (Variables|Default|SetisOn true)
    (bind _asbp_pan (Utilities|Casting|CastToBP_pan _onkompor))
    (Variables|/Game/Level/Blueprints/BP_pan.BP_pan_C|SetdiatasKompor _asbp_pan true)
    (elif (== (Variables|Default|Getheat%20level) 1)
      (Variables|Default|Setheat%20level 2)
      (goto _label)
      (elif (== (Variables|Default|Getheat%20level) 2)
        (Variables|Default|Setheat%20level 3)
        (goto _label)
        (elif (== (Variables|Default|Getheat%20level) 3)
          (Variables|Default|Setheat%20level 0)
          (Default|Change _heatlevelwg (Variables|Default|Getheat%20level))
          (Variables|Default|SetisOn false)
          (bind _asbp_pan_2 (Utilities|Casting|CastToBP_pan _onkompor))
          (Variables|/Game/Level/Blueprints/BP_pan.BP_pan_C|SetdiatasKompor _asbp_pan_2 false))))))

(event Custom|active
  (bind _returnvalue (Transformation|GetActorLocation))
  (bind _actors_to_ignore (Variables|Default|GetActors%20to%20Ignore))
  (bind (_outhit _returnvalue_2) (Collision|SphereTraceForObjects _returnvalue _returnvalue 1e+02 (Variables|Default|GetObject%20Types) false _actors_to_ignore "ForDuration"))
  (if _returnvalue_2
    (bind _output_get (Variables|Default|SetHit%20Actor (.HitActor (Collision|BreakHitResult _outhit))))
    (bind _asbp_pan (Utilities|Casting|CastToBP_pan _output_get)
      (:then
        (Variables|Default|SetonKompor _output_get :!label _label)
        (if (Variables|Default|Getgrill?)
          _
          (else
            (Transformation|SetWorldLocationAndRotation (Variables|/Game/Level/Blueprints/BP_pan.BP_pan_C|Getpan _asbp_pan) (+ (Transformation|GetActorLocation) "0.000000,0.000000,20.000000") (Transformation|GetWorldRotation (Variables|Default|GetCube)) false false)
            (Physics|SetSimulatePhysics (Variables|/Game/Level/Blueprints/BP_pan.BP_pan_C|Getpan _asbp_pan) false)))
        (bind _asbp_pan_2 (Utilities|Casting|CastToBP_pan (Variables|Default|GetonKompor))
          (:then
            (if (Variables|Default|GetisOn)
              (Default|Cook _asbp_pan_2 (Math|Conversions|ToFloat(Integer) (Variables|Default|Getheat%20level)))))
          (:CastFailed
            (bind _asbp_steak (Utilities|Casting|CastToBP_steak (Variables|Default|GetonKompor)))
            (if (Variables|Default|GetisOn)
              (Default|Cook _asbp_steak (Math|Conversions|ToFloat(Integer) (Variables|Default|Getheat%20level)))))))
      (:CastFailed
        (Utilities|Casting|CastToBP_steak _output_get
          (:then
            (goto _label))
          (:CastFailed
            (Utilities|Array|Add _actors_to_ignore (.HitActor (Collision|BreakHitResult _outhit)))))))))

(event EventBeginPlay
  (bind _returnvalue (UserInterface|CreateWidget "/Game/Level/UI/wg_cookbar.wg_cookbar_C"))
  (UserInterface|SetWidget (Variables|Default|GetWidget) _returnvalue)
  (Variables|Default|Setwg_bar _returnvalue))

(event Collision|EventActorBeginOverlap
  (params (OtherActor :type Actor%20Object%20Reference)))

(event EventTick
  (params (DeltaSeconds :type Float%20%28single-precision%29))
  (bind _onkompor (Variables|Default|GetonKompor))
  (Utilities|IsValid _onkompor
    (:Is%20Valid
      (bind _asbp_pan (Utilities|Casting|CastToBP_pan _onkompor))
      (if (> (Utilities|Array|Length (Variables|/Game/Level/Blueprints/BP_pan.BP_pan_C|Getfoodvalue _asbp_pan)) 0)
        (Default|Update (Variables|Default|Getwg_bar) (/ (.cookvalue (Utilities|Struct|Breakstrruct_food (Utilities|Array|Get(acopy) (Variables|/Game/Level/Blueprints/BP_pan.BP_pan_C|Getfoodvalue _asbp_pan)))) 1e+02))))))

(fn ConstructionScript)