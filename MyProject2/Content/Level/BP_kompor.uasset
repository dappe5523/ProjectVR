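; BP_kompor is a stove ("kompor") that holds a BP_pan and tells it whether it sits on a lit burner.
; Box overlap runs a sphere trace, stores a found pan as OnKompor, snaps it above the stove and adds other hits to an ignore list.
; The togglekompor event flip-flops IsOn and updates the pan's DiatasKompor flag.
; Pan physics follows IsOn only at overlap time, and end overlap does nothing.
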(event OnComponentBeginOverlap(Box)
  (params (OverlappedComponent :type Primitive%20Component%20Object%20Reference) (OtherActor :type Actor%20Object%20Reference) (OtherComp :type Primitive%20Component%20Object%20Reference) (OtherBodyIndex :type Integer) (bFromSweep :type Boolean) (SweepResult :type Hit%20Result%20Structure%20%28by%20ref%29))
  (bind _returnvalue (Transformation|GetActorLocation))
  (bind _actors_to_ignore (Variables|Default|GetActors%20to%20Ignore))
  (bind (_outhit _returnvalue_2) (Collision|SphereTraceForObjects _returnvalue _returnvalue 1e+02 (Variables|Default|GetObject%20Types) false _actors_to_ignore "None"))
  (if _returnvalue_2
    (bind _output_get (Variables|Default|SetHit%20Actor (.HitActor (Collision|BreakHitResult _outhit))))
    (bind _asbp_pan (Utilities|Casting|CastToBP_pan _output_get)
      (:then
        (Variables|Default|SetonKompor _output_get)
        (Transformation|SetWorldLocation (Variables|/Game/Level/BP_pan.BP_pan_C|Getpan _asbp_pan) (+ (Transformation|GetActorLocation) "0.000000,0.000000,20.000000") false false)
        (if (Variables|Default|GetisOn)
          (bind _asbp_pan_2 (Utilities|Casting|CastToBP_pan (Variables|Default|GetonKompor)))
          (Variables|/Game/Level/BP_pan.BP_pan_C|SetdiatasKompor _asbp_pan_2 true)
          (Physics|SetSimulatePhysics (Variables|/Game/Level/BP_pan.BP_pan_C|Getpan _asbp_pan) false)
          (else
            (bind _asbp_pan_3 (Utilities|Casting|CastToBP_pan (Variables|Default|GetonKompor)))
            (Variables|/Game/Level/BP_pan.BP_pan_C|SetdiatasKompor _asbp_pan_3 false)
            (Physics|SetSimulatePhysics (Variables|/Game/Level/BP_pan.BP_pan_C|Getpan _asbp_pan) true))))
      (:CastFailed
        (Utilities|Array|Add _actors_to_ignore (.HitActor (Collision|BreakHitResult _outhit)))))))

(event OnComponentEndOverlap(Box)
  (params (OverlappedComponent :type Primitive%20Component%20Object%20Reference) (OtherActor :type Actor%20Object%20Reference) (OtherComp :type Primitive%20Component%20Object%20Reference) (OtherBodyIndex :type Integer)))

(event Custom|togglekompor
  (bind _onkompor (Variables|Default|GetonKompor))
  (Utilities|FlowControl|FlipFlop
    (:A
      (Variables|Default|SetisOn true)
      (Development|PrintString "on")
      (bind _asbp_pan (Utilities|Casting|CastToBP_pan _onkompor))
      (Variables|/Game/Level/BP_pan.BP_pan_C|SetdiatasKompor _asbp_pan true)
      (Development|PrintString "on"))
    (:B
      (Variables|Default|SetisOn false)
      (Development|PrintString "off")
      (bind _asbp_pan_2 (Utilities|Casting|CastToBP_pan _onkompor))
      (Variables|/Game/Level/BP_pan.BP_pan_C|SetdiatasKompor _asbp_pan_2 false)
      (Development|PrintString "off"))))

(event EventBeginPlay)

(event Collision|EventActorBeginOverlap
  (params (OtherActor :type Actor%20Object%20Reference)))

(event EventTick
  (params (DeltaSeconds :type Float%20%28single-precision%29)))

(fn ConstructionScript)